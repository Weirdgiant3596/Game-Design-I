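; Patrol AI pawn that walks between actors tagged as BunkerMap patrol points in random order.
; BeginPlay gathers and shuffles the points and randomizes walk speed, then starts an AIMoveTo loop that advances after a short delay on success or failure.
; The list reshuffles after each full pass.
; A separate GotoDesination event repeatedly moves to the player, but nothing in this graph starts it.
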(event Custom|GoToPatrolPoints
  (AI|AIMoveTo self (Transformation|GetActorLocation (Utilities|Array|Get(acopy) (stale EventBeginPlay _outactors) (Variables|Default|GetCurrentPatrolPoint))) 0 1e+02 false
    (:OnSuccess
      (Development|PrintString "Arrived at Destination"))
    (:OnFail
      (Development|PrintString "Failed to get to Desination" true true "(R=0.541667,G=0.000000,B=0.006783,A=1.000000)")))
  (bind _result (Math|Integer|IncrementInt (Variables|Default|GetCurrentPatrolPoint))
    (:%20%20
      (if (>= _result (Utilities|Array|Length (stale EventBeginPlay _outactors)))
        (Variables|Default|SetCurrentPatrolPoint 0)
        (Utilities|Array|Shuffle (stale EventBeginPlay _outactors)))
      (Utilities|FlowControl|Delay 1.0)
      (CallFunction|GotoPatrolPoints))))

(event Custom|Go%20to%20Desination
  (AI|AIMoveTo self "0, 0, 0" (Game|GetPlayerCharacter 0) 2e+02 false
    (:OnSuccess
      (Development|PrintString "Arrived at Destination"))
    (:OnFail
      (Development|PrintString "Failed to get to Desination" true true "(R=0.541667,G=0.000000,B=0.006783,A=1.000000)")))
  (Utilities|FlowControl|Delay 1.0)
  (CallFunction|GotoDesination))

(event EventBeginPlay
  (bind _outactors (Actor|GetAllActorsOfClasswithTag "/Script/Engine.Actor" "PatrolPoint - BunkerMap"))
  (Development|PrintString (Utilities|String|Append "There are " (Utilities|String|ToString(Integer) (Utilities|Array|Length _outactors)) " patrol points."))
  (Utilities|Array|Shuffle _outactors)
  (Variables|/Script/Engine.CharacterMovementComponent|SetMaxWalkSpeed (Variables|Character|GetCharacterMovement) (Math|Conversions|ToFloat(Integer) (* (Math|Random|RandomIntegerinRange 8 12) 25)))
  (CallFunction|GotoPatrolPoints))

(fn ConstructionScript)