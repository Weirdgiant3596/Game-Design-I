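; BP_SlidingDoor is a double sliding door that opens when the custom third-person character enters its trigger box.
; A Timeline lerps each door panel's relative location between its start and end marker components.
; Any actor leaving the box reverses the Timeline to close the door, as the end-overlap event has no character check.
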(event OnComponentEndOverlap(Box)
  (params (OverlappedComponent :type Primitive%20Component%20Object%20Reference) (OtherActor :type Actor%20Object%20Reference) (OtherComp :type Primitive%20Component%20Object%20Reference) (OtherBodyIndex :type Integer))
  (bind (_direction _leftdoor _rightdoor) (Timeline|Timeline Reverse)
    (:Update
      (Transformation|SetRelativeLocation (Variables|Default|GetLeftDoor) (Math|Vector|Lerp(Vector) (Variables|/Script/Engine.SceneComponent|GetRelativeLocation (Variables|Default|GetLeftStart)) (Variables|/Script/Engine.SceneComponent|GetRelativeLocation (Variables|Default|GetLeftEnd)) _leftdoor) false false)
      (Transformation|SetRelativeLocation (Variables|Default|GetRightDoor) (Math|Vector|Lerp(Vector) (Variables|/Script/Engine.SceneComponent|GetRelativeLocation (Variables|Default|GetRightStart)) (Variables|/Script/Engine.SceneComponent|GetRelativeLocation (Variables|Default|GetRightEnd)) _rightdoor) false false))))

(event OnComponentBeginOverlap(Box)
  (params (OverlappedComponent :type Primitive%20Component%20Object%20Reference) (OtherActor :type Actor%20Object%20Reference) (OtherComp :type Primitive%20Component%20Object%20Reference) (OtherBodyIndex :type Integer) (bFromSweep :type Boolean) (SweepResult :type Hit%20Result%20Structure%20%28by%20ref%29))
  (Utilities|Casting|CastToBP_ThirdPersonCharacterCustom OtherActor)
  (bind (_direction _leftdoor _rightdoor) (Timeline|Timeline Play)
    (:Update
      (Transformation|SetRelativeLocation (Variables|Default|GetLeftDoor) (Math|Vector|Lerp(Vector) (Variables|/Script/Engine.SceneComponent|GetRelativeLocation (Variables|Default|GetLeftStart)) (Variables|/Script/Engine.SceneComponent|GetRelativeLocation (Variables|Default|GetLeftEnd)) _leftdoor) false false)
      (Transformation|SetRelativeLocation (Variables|Default|GetRightDoor) (Math|Vector|Lerp(Vector) (Variables|/Script/Engine.SceneComponent|GetRelativeLocation (Variables|Default|GetRightStart)) (Variables|/Script/Engine.SceneComponent|GetRelativeLocation (Variables|Default|GetRightEnd)) _rightdoor) false false))))

(event EventBeginPlay)

(event EventTick
  (params (DeltaSeconds :type Float%20%28single-precision%29)))

(fn ConstructionScript)